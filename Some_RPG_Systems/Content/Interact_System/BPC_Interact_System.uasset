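; Actor component that tracks nearby interactable actors and lets its owner interact with them, adding the target to the owner's BPC_Inventory.
; UpdatePossibleInteractions maintains the candidate list, targets the nearest, and shows or hides a lazily created WBP_Interact_Prompt.
; Debug key E triggers interaction; both arrow keys retarget to the nearest candidate other than the current one, effectively toggling between the closest two.
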(event Input|KeyboardEvents|DebugKeyE
  (params (Key :type Key%20Structure :default "None") (ActionValue :type Input%20Action%20Value%20Structure))
  (:Pressed
    (if (Variables|Default|GetCan_Interact)
      (CallFunction|Interact))))

(event Input|KeyboardEvents|DebugKeyLeft
  (params (Key :type Key%20Structure :default "None") (ActionValue :type Input%20Action%20Value%20Structure))
  (:Pressed
    (CallFunction|SwitchCurrentInteraction)))

(event Input|KeyboardEvents|DebugKeyRight
  (params (Key :type Key%20Structure :default "None") (ActionValue :type Input%20Action%20Value%20Structure))
  (:Pressed
    (CallFunction|SwitchCurrentInteraction)))

(fn Interact
  (bind _current_interaction (Variables|Default|GetCurrent_Interaction))
  (Class|BPICanInteractwith|Interact(Message) _current_interaction)
  (Development|PrintString (Utilities|GetDisplayName _current_interaction))
  (Default|AddtoInventory (Actor|GetComponentbyClass (Components|GetOwner) "/Game/Inventory_System/BPC_Inventory.BPC_Inventory_C") (Variables|Default|GetCurrent_Interaction)))

(fn UpdatePossibleInteractions
  (params (New_Interaction :type Actor%20Object%20Reference) (Adding? :type Boolean))
  (if Adding?
    (Utilities|Array|Add (Variables|Default|GetPossible_Interactions) New_Interaction)
    (else
      (Utilities|Array|RemoveItem (Variables|Default|GetPossible_Interactions) New_Interaction)))
  (Variables|Default|SetCurrent_Interaction (.ReturnValue (Actor|FindNearestActor (Transformation|GetActorLocation (Components|GetOwner)) (Variables|Default|GetPossible_Interactions))))
  (if (Utilities|Array|IsEmpty (Variables|Default|GetPossible_Interactions))
    (CallFunction|UpdateVisibilityInteractPrompt false)
    (else
      (CallFunction|UpdateVisibilityInteractPrompt true))))

(fn SwitchCurrentInteraction
  (bind _output_get (LocalVariables|SetLocal_Possible_Interactions (Variables|Default|GetPossible_Interactions)))
  (Utilities|Array|RemoveItem _output_get (Variables|Default|GetCurrent_Interaction))
  (Variables|Default|SetCurrent_Interaction (.ReturnValue (Actor|FindNearestActor (Transformation|GetActorLocation (Components|GetOwner)) (LocalVariables|GetLocal_Possible_Interactions))))
  (Default|UpdateCurrentInteractionName (Variables|Default|GetInteract_Prompt_Ref)))

(fn UpdateVisibilityInteractPrompt
  (params (Visible? :type Boolean))
  (if Visible?
    (Utilities|IsValid (Variables|Default|GetInteract_Prompt_Ref)
      (:Is%20Valid
        (Widget|SetVisibility (Variables|Default|GetInteract_Prompt_Ref) "Visible"))
      (:Is%20Not%20Valid
        (bind _returnvalue (UserInterface|CreateWidget "/Game/Interact_System/WBP_Interact_Prompt.WBP_Interact_Prompt_C"))
        (bind _output_get (Variables|Default|SetInteract_Prompt_Ref _returnvalue))
        (UserInterface|Viewport|AddtoViewport _output_get 0)))
    (Variables|Default|SetCan_Interact true)
    (Default|UpdateCurrentInteractionName (Variables|Default|GetInteract_Prompt_Ref))
    (else
      (Widget|SetVisibility (Variables|Default|GetInteract_Prompt_Ref) "Hidden")
      (Variables|Default|SetCan_Interact false))))