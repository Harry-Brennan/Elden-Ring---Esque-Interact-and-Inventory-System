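; Inventory component that holds item actors and manages the owner's left and right weapons and four armour slots.
; Stored items stay in the world, moved to random reachable navmesh points inside a storage area rather than destroyed.
; Equipping attaches items to named owner sockets, with armour slots indexed by type, while dropping uses a short forward trace to place them.
; A debug Tab key toggles the WBP_Inventory widget.
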(event Input|KeyboardEvents|DebugKeyTab
  (params (Key :type Key%20Structure :default "None") (ActionValue :type Input%20Action%20Value%20Structure))
  (:Pressed
    (Utilities|FlowControl|FlipFlop
      (:A
        (bind _returnvalue (UserInterface|CreateWidget "/Game/Inventory_System/WBP_Inventory.WBP_Inventory_C" (Game|GetPlayerController 0)))
        (bind _output_get (Variables|UI|SetInventory_Ref _returnvalue))
        (UserInterface|Viewport|AddtoViewport _output_get 0))
      (:B
        (Widget|RemovefromParent (Variables|UI|GetInventory_Ref))))))

(fn AddtoInventory
  (params (ToAdd :type Actor%20Object%20Reference))
  (Utilities|Array|Add (Variables|Inventory|GetInventory) ToAdd)
  (Transformation|SetActorLocation ToAdd (.RandomLocation (AI|Navigation|GetRandomReachablePointinRadius (Variables|StorageAreaInfo|GetCentreOfStorageArea) (Variables|StorageAreaInfo|GetStorageAreaRadius) 0 0)) false true))

(fn Remove
  (params (ToRemove :type Actor%20Object%20Reference))
  (Utilities|Array|RemoveItem (Variables|Inventory|GetInventory) ToRemove))

(fn UpdateWeapon
  (params (NewWeapon :type Actor%20Object%20Reference) (RightHand? :type Boolean))
  (Utilities|IsValid (select RightHand? (Variables|CurrentEquipment|GetCurrentWeaponRight) (Variables|CurrentEquipment|GetCurrentWeaponLeft))
    (:Is%20Valid
      (CallFunction|UnequipWeapon (select RightHand? (Variables|CurrentEquipment|GetCurrentWeaponRight) (Variables|CurrentEquipment|GetCurrentWeaponLeft)) false))
    (:Is%20Not%20Valid
      _))
  (if RightHand?
    (Variables|CurrentEquipment|SetCurrentWeaponRight NewWeapon)
    (CallFunction|EquipWeapon NewWeapon true)
    (else
      (Variables|CurrentEquipment|SetCurrentWeaponLeft NewWeapon)
      (CallFunction|EquipWeapon NewWeapon false))))

(fn UpdateArmour
  (params (NewArmour :type Actor%20Object%20Reference))
  (bind _armourtype (Class|BPIArmour|GetArmourType(Message) NewArmour))
  (Utilities|IsValid (Utilities|Array|Get(acopy) (Variables|Inventory|GetInventory) _armourtype)
    (:Is%20Valid
      (CallFunction|UnequipArmourPiece (Utilities|Array|Get(acopy) (Variables|Inventory|GetInventory) _armourtype))
      (CallFunction|EquipArmourPiece NewArmour))
    (:Is%20Not%20Valid
      (Utilities|Array|SetArrayElem (Variables|CurrentEquipment|GetCurrentArmour) _armourtype NewArmour)
      (CallFunction|EquipArmourPiece NewArmour))))

(fn DropWeapon
  (params (WeaponToDrop :type Actor%20Object%20Reference) (IsEquipped? :type Boolean) (%28if_equipped%29RightHand? :type Boolean))
  (bind _returnvalue (Components|GetOwner))
  (bind _returnvalue_2 (Transformation|GetActorLocation _returnvalue))
  (Transformation|DetachFromActor WeaponToDrop "KeepRelative" "KeepRelative" "KeepRelative")
  (bind (_outhit _returnvalue_3) (Collision|LineTraceForObjects _returnvalue_2 (+ _returnvalue_2 (* (Transformation|GetActorForwardVector _returnvalue) 25.0)) (Utilities|Array|MakeArray "ObjectTypeQuery1" "ObjectTypeQuery2") false (Utilities|Array|MakeArray (Components|GetOwner)) "ForDuration"))
  (Transformation|SetActorLocation WeaponToDrop (Math|Vector|SelectVector (.Location (Collision|BreakHitResult _outhit)) (.TraceEnd (Collision|BreakHitResult _outhit)) _returnvalue_3) false true)
  (if IsEquipped?
    (CallFunction|UnequipWeapon WeaponToDrop %28if_equipped%29RightHand?)
    (else
      (CallFunction|Remove WeaponToDrop))))

(fn DropArmourPiece
  (params (ArmourPieceToDrop :type Actor%20Object%20Reference))
  (bind _returnvalue (Components|GetOwner))
  (bind _returnvalue_2 (Transformation|GetActorLocation _returnvalue))
  (Transformation|DetachFromActor ArmourPieceToDrop "KeepRelative" "KeepRelative" "KeepRelative")
  (bind (_outhit _returnvalue_3) (Collision|LineTraceForObjects _returnvalue_2 (+ _returnvalue_2 (* (Transformation|GetActorForwardVector _returnvalue) 25.0)) (Utilities|Array|MakeArray "ObjectTypeQuery1" "ObjectTypeQuery2") false (Utilities|Array|MakeArray (Components|GetOwner)) "ForDuration"))
  (Transformation|SetActorLocation ArmourPieceToDrop (Math|Vector|SelectVector (.Location (Collision|BreakHitResult _outhit)) (.TraceEnd (Collision|BreakHitResult _outhit)) _returnvalue_3) false true)
  (if (Utilities|Array|ContainsItem (Variables|CurrentEquipment|GetCurrentArmour) ArmourPieceToDrop)
    (CallFunction|UnequipArmourPiece ArmourPieceToDrop)
    (else
      (CallFunction|Remove ArmourPieceToDrop))))

(fn UnequipWeapon
  (params (WeaponToUnequip :type Actor%20Object%20Reference) (RightHand? :type Boolean))
  (if RightHand?
    (Variables|CurrentEquipment|SetCurrentWeaponRight 0)
    (else
      (Variables|CurrentEquipment|SetCurrentWeaponLeft 0)))
  (Transformation|SetActorLocation WeaponToUnequip (.RandomLocation (AI|Navigation|GetRandomReachablePointinRadius (Variables|StorageAreaInfo|GetCentreOfStorageArea) (Variables|StorageAreaInfo|GetStorageAreaRadius) 0 0)) false false))

(fn UnequipArmourPiece
  (params (ArmourPieceToUnequip :type Actor%20Object%20Reference))
  (bind _armourtype (Class|BPIArmour|GetArmourType(Message) ArmourPieceToUnequip))
  (Transformation|DetachFromActor (Utilities|Array|Get(acopy) (Variables|CurrentEquipment|GetCurrentArmour) _armourtype) "KeepRelative" "KeepRelative" "KeepRelative")
  (Transformation|SetActorLocation (Utilities|Array|Get(acopy) (Variables|CurrentEquipment|GetCurrentArmour) _armourtype) (.RandomLocation (AI|Navigation|GetRandomReachablePointinRadius (Variables|StorageAreaInfo|GetCentreOfStorageArea) (Variables|StorageAreaInfo|GetStorageAreaRadius) 0 0)) false false)
  (Utilities|Array|SetArrayElem (Variables|CurrentEquipment|GetCurrentArmour) _armourtype 0))

(fn EquipWeapon
  (params (WeaponToEquip :type Actor%20Object%20Reference) (RightHand? :type Boolean))
  (Transformation|AttachActorToActor WeaponToEquip (Components|GetOwner) (select RightHand? (Variables|Bones|GetRightHandBoneName) (Variables|Bones|GetLeftHandBoneName)) "KeepRelative" "KeepRelative" "KeepRelative" true))

(fn EquipArmourPiece
  (params (ArmourPieceToEquip :type Actor%20Object%20Reference))
  (bind _armourtype (Class|BPIArmour|GetArmourType(Message) ArmourPieceToEquip))
  (switch int _armourtype
    (:Default
      (Development|PrintString "INVALID ARMOUR TYPE"))
    (:0
      ;[1 1 1] Head piece
      (Transformation|AttachActorToActor ArmourPieceToEquip (Components|GetOwner) (Variables|Bones|GetHeadBoneName) "KeepRelative" "KeepRelative" "KeepRelative" true))
    (:1
      ;[1 1 1] Chest armour
      (Transformation|AttachActorToActor ArmourPieceToEquip (Components|GetOwner) (Variables|Bones|GetChestBoneName) "KeepRelative" "KeepRelative" "KeepRelative" true))
    (:2
      ;[1 1 1] Gauntlets
      (Transformation|AttachActorToActor ArmourPieceToEquip (Components|GetOwner) (Variables|Bones|GetRightArmBoneName) "KeepRelative" "KeepRelative" "KeepRelative" true)
      (Transformation|AttachActorToActor ArmourPieceToEquip (Components|GetOwner) (Variables|Bones|GetLeftArmBoneName) "KeepRelative" "KeepRelative" "KeepRelative" true))
    (:3
      ;[1 1 1] Leg armour
      (Transformation|AttachActorToActor ArmourPieceToEquip (Components|GetOwner) (Variables|Bones|GetRightLegBoneName) "KeepRelative" "KeepRelative" "KeepRelative" true)
      (Transformation|AttachActorToActor ArmourPieceToEquip (Components|GetOwner) (Variables|Bones|GetLeftLegBoneName) "KeepRelative" "KeepRelative" "KeepRelative" true))))