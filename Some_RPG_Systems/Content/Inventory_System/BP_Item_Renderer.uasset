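; BP_Item_Renderer is an inventory system actor that renders an isolated, rotatable view of an item's static mesh.
; On BeginPlay it sets the Renderer's show-only list to itself, so the capture excludes the rest of the world.
; UpdateItemStaticMesh swaps the mesh, resets the spring arm's rotation and prints a debug string.
; RotateMesh turns 2D input into scaled, inverted pitch and yaw on the spring arm, leaving the mesh itself still.
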(event EventBeginPlay
  (Variables|/Script/Engine.SceneCaptureComponent|SetShowOnlyActors (Variables|Default|GetRenderer) (Utilities|Array|MakeArray self)))

(fn ConstructionScript)

(fn UpdateItemStaticMesh
  (params (NewStaticMesh :type Static%20Mesh%20Object%20Reference))
  (Components|StaticMesh|SetStaticMesh (Variables|Default|GetItem_Static_Mesh) NewStaticMesh)
  (Transformation|SetRelativeRotation (Variables|Default|GetRendererSpringArm) "0, 0, 0" false false)
  (Development|PrintString "UPDATED ITEM MESH"))

(fn RotateMesh
  (params (XYRot :type Vector%202D%20Structure))
  (bind (_x _y) (Math|Vector2D|BreakVector2D XYRot))
  (Transformation|AddLocalRotation (Variables|Default|GetRendererSpringArm) (Math|Rotator|MakeRotator 0.0 (* _y -1.5) (* _x -1.5)) false false))