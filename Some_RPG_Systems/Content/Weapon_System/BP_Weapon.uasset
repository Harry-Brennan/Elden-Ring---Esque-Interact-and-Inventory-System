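; BP_Weapon is a weapon actor that the player can pick up as a world item or hold as equipped.
; An interaction sphere, sized in the construction script, adds or removes the weapon from the player's BPC_Interact_System on overlap.
; The equipped flag switches actor collision and mesh physics off when equipped and on when loose.
; Getters expose name, mesh, display info, storage type and equipped status; the image getter returns nothing.
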(event OnComponentBeginOverlap(InteractCollision)
  (params (OverlappedComponent :type Primitive%20Component%20Object%20Reference) (OtherActor :type Actor%20Object%20Reference) (OtherComp :type Primitive%20Component%20Object%20Reference) (OtherBodyIndex :type Integer) (bFromSweep :type Boolean) (SweepResult :type Hit%20Result%20Structure%20%28by%20ref%29))
  (if (== OtherActor (Game|GetPlayerCharacter 0))
    (Default|UpdatePossibleInteractions (Actor|GetComponentbyClass OtherActor "/Game/Interact_System/BPC_Interact_System.BPC_Interact_System_C") self true)))

(event OnComponentEndOverlap(InteractCollision)
  (params (OverlappedComponent :type Primitive%20Component%20Object%20Reference) (OtherActor :type Actor%20Object%20Reference) (OtherComp :type Primitive%20Component%20Object%20Reference) (OtherBodyIndex :type Integer))
  (if (== OtherActor (Game|GetPlayerCharacter 0))
    (Default|UpdatePossibleInteractions (Actor|GetComponentbyClass OtherActor "/Game/Interact_System/BPC_Interact_System.BPC_Interact_System_C") self false)))

(event EventUpdateEquippedCollision
  (params (Equipped? :type Boolean))
  (bind _output_get (Variables|Default|SetEquipped? Equipped?))
  (if _output_get
    (Collision|SetActorEnableCollision false)
    (CallFunction|UpdatePhysics false)
    (else
      (Collision|SetActorEnableCollision true)
      (CallFunction|UpdatePhysics true))))

(event EventBeginPlay
  (CallFunction|UpdateEquippedCollision (Variables|Default|GetEquipped?)))

(event EventUpdatePhysics
  (params (Enabled? :type Boolean))
  (if Enabled?
    (Physics|SetSimulatePhysics (Variables|Default|GetWeaponStaticMesh) true)
    (else
      (Physics|SetSimulatePhysics (Variables|Default|GetWeaponStaticMesh) false))))

(fn ConstructionScript
  (Components|Sphere|SetSphereRadius (Variables|Default|GetInteractCollision) (Variables|Default|GetInteract_Collision_Radius) true))

(fn GetEquippedStatus
  (return (Variables|Default|GetEquipped?)))

(fn GetImageRepresentation
  (return 0))

(fn GetInfoforDisplay
  (return (Variables|Default|GetDisplayed_Item_Info) ""))

(fn GetItemMesh
  (return (Variables|/Script/Engine.StaticMeshComponent|GetStaticMesh (Variables|Default|GetWeaponStaticMesh))))

(fn GetName
  (return (Variables|Default|GetWeapon_Name)))

(fn GetNameforStorage
  (return (Variables|Default|GetWeapon_Name)))

(fn GetTypeforStorage
  (return (Variables|Default|GetStorage_Type)))